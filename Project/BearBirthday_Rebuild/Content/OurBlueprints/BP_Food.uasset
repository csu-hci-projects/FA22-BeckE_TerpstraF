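; BP_Food is a VR food pickup that spins to show it is collectable.
; A looping timer rotates its GrabComponent in yaw from BeginPlay onward.
; Grabbing it increments the VRPawn's Consumed count and lowers Exhaustion, clamped at zero.
; It then flags the pawn as ConsumingFood for a few seconds before clearing the flag and destroying itself.
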(event OnGrabbed(GrabComponent)
  ;[1 1 1] Increase Consumed Count
  (bind _asvrpawn (Utilities|Casting|CastToVRPawn (Game|Player|GetPlayerPawn 0)))
  (Variables|/Game/VRTemplate/Blueprints/VRPawn.VRPawn_C|Setconsumed _asvrpawn (+ (Variables|/Game/VRTemplate/Blueprints/VRPawn.VRPawn_C|Getconsumed _asvrpawn) 1))
  ;[1 1 1] Reduce Exhaustion
  (if (< (Variables|/Game/VRTemplate/Blueprints/VRPawn.VRPawn_C|GetExhaustion _asvrpawn) 0.11)
    (Variables|/Game/VRTemplate/Blueprints/VRPawn.VRPawn_C|SetExhaustion _asvrpawn 0.0)
    (else
      (Variables|/Game/VRTemplate/Blueprints/VRPawn.VRPawn_C|SetExhaustion _asvrpawn (- (Variables|/Game/VRTemplate/Blueprints/VRPawn.VRPawn_C|GetExhaustion _asvrpawn) 0.11))))
  ;[1 1 1] Eat Food Timer
  (Variables|/Game/VRTemplate/Blueprints/VRPawn.VRPawn_C|SetConsumingFood _asvrpawn true)
  (Utilities|FlowControl|Delay 5.0)
  (Variables|/Game/VRTemplate/Blueprints/VRPawn.VRPawn_C|SetConsumingFood _asvrpawn false)
  (Actor|DestroyActor))

(event EventBeginPlay
  ;[1 1 1] Rotate Item (to show collectable status)
  (Utilities|Time|SetTimerbyFunctionName 0 "Rotate" 0.005 true))

(fn ConstructionScript)

(fn Rotate
  (Transformation|AddLocalRotation (Variables|Default|GetGrabComponent) (Math|Rotator|MakeRotator 0.0 0.0 0.5) false false))